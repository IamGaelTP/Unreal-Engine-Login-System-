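; Game instance that sets up PlayFab on Init and handles email login, account registration and password recovery.
; Successful login opens LevelSuccess; registration and recovery successes report through widget text or a debug print.
; A shared Failure handler prints the error and writes it to a BP_SignUpLoginPage status field chosen by panel visibility.
; Failure and post-registration field clearing act on newly created widgets that are never added to the viewport.
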(event `self.ReceiveInit`
  ;[1 0.8878 0.1282] INIT PLAYFAB
  (`PlayFabUtilities.setPlayFabSettings` "C1DDC")
  (`KismetSystemLibrary.PrintString` "PlayFab Setter"))

(event `Login`
  (params (Email :type String) (Password :type String))
  ;[0.8052 0.5759 0.257] Login and register
  ;;[0.3578 1 0.5591] On Success
  (`PlayFabClientAPI.LoginWithEmailAddress` (make `ClientLoginWithEmailAddressRequest` null Email null Password) (delegate `LoginSuccess`) (delegate `Failure`)))

(event `Failure`
  (params (error :type "PlayFabError Structure") (customData :type "Object Object Reference"))
  (bind _returnvalue (`KismetStringLibrary.Concat_StrStr` (`KismetStringLibrary.Conv_IntToString` error_ErrorCode) error_ErrorName error_ErrorMessage error_ErrorDetails))
  (bind _returnvalue_2 (`KismetTextLibrary.Conv_StringToText` _returnvalue))
  ;[0.8052 0.5759 0.257] Login and register
  ;;[1 0.149 0.149] On Failure
  (`KismetSystemLibrary.PrintString` _returnvalue)
  (bind _returnvalue_3 (`|CreateWidget` "/Game/UI/Blueprints/BP_SignUpLoginPage.BP_SignUpLoginPage_C"))
  (if (`KismetMathLibrary.Conv_IntToBool` (`KismetMathLibrary.Conv_ByteToInt` (`Widget.GetVisibility` (`/Game/UI/Blueprints/BP_SignUpLoginPage.CanvasPanel_Login` _returnvalue_3))))
    (bind _returnvalue_4 (`|CreateWidget` "/Game/UI/Blueprints/BP_SignUpLoginPage.BP_SignUpLoginPage_C"))
    (`TextBlock.SetText` (`/Game/UI/Blueprints/BP_SignUpLoginPage.LoginStatusText` _returnvalue_4) _returnvalue_2)
    (elif (`KismetMathLibrary.Conv_IntToBool` (`KismetMathLibrary.Conv_ByteToInt` (`Widget.GetVisibility` (`/Game/UI/Blueprints/BP_SignUpLoginPage.CanvasPanel_SignUp` _returnvalue_3))))
      (bind _returnvalue_5 (`|CreateWidget` "/Game/UI/Blueprints/BP_SignUpLoginPage.BP_SignUpLoginPage_C"))
      (`TextBlock.SetText` (`/Game/UI/Blueprints/BP_SignUpLoginPage.StatusTextBox` _returnvalue_5) _returnvalue_2)
      (elif (`KismetMathLibrary.Conv_IntToBool` (`KismetMathLibrary.Conv_ByteToInt` (`Widget.GetVisibility` (`/Game/UI/Blueprints/BP_SignUpLoginPage.CanvasPanel_sendpassreset` _returnvalue_3))))
        (bind _returnvalue_6 (`|CreateWidget` "/Game/UI/Blueprints/BP_SignUpLoginPage.BP_SignUpLoginPage_C"))
        (`TextBlock.SetText` (`/Game/UI/Blueprints/BP_SignUpLoginPage.passemailTextBlock` _returnvalue_6) _returnvalue_2)
        (else
          (`KismetSystemLibrary.PrintString` "Canvas is Hidden!"))))))

(event `LoginSuccess`
  (params (result :type "ClientLoginResult Structure") (customData :type "Object Object Reference"))
  ;[0.8052 0.5759 0.257] Login and register
  ;;[0.3578 1 0.5591] On Success
  (`GameplayStatics.OpenLevel` "LevelSuccess" :!pinned true) ; Init Game
)

(event `Register`
  (params (`Display Name` :type String) (Email :type String) (Password :type String) (Username :type String))
  ;[0.8052 0.5759 0.257] Login and register
  ;;[0.3578 1 0.5591] On Success
  (`PlayFabClientAPI.RegisterPlayFabUser` (make `ClientRegisterPlayFabUserRequest` null `Display Name` Email "" null Password "" false Username) (delegate `RegisterSuccess`) (delegate `Failure`)))

(event `RegisterSuccess`
  (params (result :type "ClientRegisterPlayFabUserResult Structure") (customData :type "Object Object Reference"))
  ;[0.8052 0.5759 0.257] Login and register
  ;;[0.3578 1 0.5591] On Success
  (bind _asbp_sign_up_login_page (cast `/Game/UI/Blueprints/BP_SignUpLoginPage` customData)
    (:`then`
      (bind _statustextbox (`/Game/UI/Blueprints/BP_SignUpLoginPage.StatusTextBox` _asbp_sign_up_login_page))
      (`/Engine/EditorBlueprintResources/StandardMacros.IsValid` _statustextbox
        (:`Is Valid`
          (`TextBlock.SetText` _statustextbox "Register Successfull")
          (`|ExecutionSequence`
            (:`then_0`
              (`KismetSystemLibrary.Delay` 2.0))
            (:`then_1`
              (`KismetSystemLibrary.Delay` 2.5))
            (:`then_2`
              (`KismetSystemLibrary.Delay` 3.0)))
          (bind _returnvalue (`|CreateWidget` "/Game/UI/Blueprints/BP_SignUpLoginPage.BP_SignUpLoginPage_C"))
          (`|ExecutionSequence`
            (:`then_0`
              (`EditableTextBox.SetText` (`/Game/UI/Blueprints/BP_SignUpLoginPage.EmailTextBox` _returnvalue) " "))
            (:`then_1`
              (`EditableTextBox.SetText` (`/Game/UI/Blueprints/BP_SignUpLoginPage.PasswordTextBox` _returnvalue) " "))
            (:`then_2`
              (`EditableTextBox.SetText` (`/Game/UI/Blueprints/BP_SignUpLoginPage.UsernameTextBox` _returnvalue) " "))))
        (:`Is Not Valid`
          (`KismetSystemLibrary.PrintString` "Doesnt Exist" :!label _label))))
    (:`CastFailed`
      (goto _label))))

(event `ForgotPassword`
  (params (Email :type String))
  ;[0.1982 0.7467 1] Forgot Password
  (`PlayFabClientAPI.SendAccountRecoveryEmail` (make `ClientSendAccountRecoveryEmailRequest` null Email) (delegate `OnResetPasswordSuccess`) (delegate `Failure`)))

(event `OnResetPasswordSuccess`
  (params (result :type "ClientSendAccountRecoveryEmailResult Structure") (customData :type "Object Object Reference"))
  ;[0.1982 0.7467 1] Forgot Password
  (`KismetSystemLibrary.PrintString` "Email has been send"))